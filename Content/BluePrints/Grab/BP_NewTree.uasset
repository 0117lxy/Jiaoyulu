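; BP_NewTree is a tree spot that starts hidden and appears as a white birch when an actor tagged "Grab" enters its Box.
; BeginPlay hides the StaticMesh, and the tagged overlap shows it, assigns the birch mesh and sets IsOverlap.
; Any end overlap clears IsOverlap but leaves the tree visible.
; Every begin overlap also prints the overlapped component's name, whatever the actor's tag.
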(event `self.ReceiveBeginPlay`
  (`SceneComponent.SetVisibility` (`self.StaticMesh`) false false))

(event `self.Box.OnComponentBeginOverlap`
  (params (OverlappedComponent :type "PrimitiveComponent Object Reference") (OtherActor :type "Actor Object Reference") (OtherComp :type "PrimitiveComponent Object Reference") (OtherBodyIndex :type Integer) (bFromSweep :type Boolean) (SweepResult :type "HitResult Structure (by ref)"))
  (bind _staticmesh (`self.StaticMesh`))
  (`KismetSystemLibrary.PrintString` (`KismetSystemLibrary.GetDisplayName` OverlappedComponent))
  (if (`self.ActorHasTag` OtherActor "Grab")
    (`SceneComponent.SetVisibility` _staticmesh true false)
    (`StaticMeshComponent.SetStaticMesh` _staticmesh "/Game/XBH_Vegetation/Mesh/white_birch/white_birch001_2.white_birch001_2")
    (set `self.Is Overlap` true)))

(event `self.Box.OnComponentEndOverlap`
  (params (OverlappedComponent :type "PrimitiveComponent Object Reference") (OtherActor :type "Actor Object Reference") (OtherComp :type "PrimitiveComponent Object Reference") (OtherBodyIndex :type Integer))
  (set `self.Is Overlap` false))

(fn `UserConstructionScript`)