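; BP_GrowTree is a tree actor that stays hidden until triggered, then appears and grows to ten times its starting scale.
; BeginPlay caches the root's world scale, computes the target and hides the mesh.
; Tick polls TimeToGrow, which this graph never sets true; while true, it shows the mesh and plays a timeline that lerps the root scale.
; The timeline clears the flag when finished.
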(event `self.ReceiveBeginPlay`
  (bind _output_get (set `self.Now Scale` (`SceneComponent.K2_GetComponentScale` (`self.DefaultSceneRoot`))))
  (set `self.Max Scale` (* _output_get 10))
  (`SceneComponent.SetVisibility` (`self.StaticMesh`) false false))

(event `self.ReceiveTick`
  (params (DeltaSeconds :type "Float (single-precision)"))
  (if (`self.Time to Grow`)
    (`SceneComponent.SetVisibility` (`self.StaticMesh`) true false)
    (bind (_direction `_新建轨道_0`) (`Timeline|时间轴_0`)
      (:`Update`
        (`SceneComponent.SetWorldScale3D` (`self.DefaultSceneRoot`) (`KismetMathLibrary.VLerp` (`self.Now Scale`) (`self.Max Scale`) `_新建轨道_0`)))
      (:`Finished`
        (set `self.Time to Grow` false)))))

(fn `UserConstructionScript`)